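; Collectable pickup that the player can grab when standing inside its box trigger.
; Overlap by the player enables input, passes the item's CollectableID to the first-person character and turns on custom depth for highlighting; leaving reverses this, sending an ID of zero.
; The HumanInteract event prints a debug message, triggers one of six grab calls on the level's audio director according to WhichItem, then destroys the actor.
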(event OnComponentBeginOverlap(Box)
  (params (OverlappedComponent :type Primitive%20Component%20Object%20Reference) (OtherActor :type Actor%20Object%20Reference) (OtherComp :type Primitive%20Component%20Object%20Reference) (OtherBodyIndex :type Integer) (bFromSweep :type Boolean) (SweepResult :type Hit%20Result%20Structure%20%28by%20ref%29))
  ;[1 1 1] Is Player At Object
  (if (== OtherActor (Game|GetPlayerCharacter 0))
    ;[1 1 1] Can Press E
    (Input|EnableInput (Game|GetPlayerController 0))
    (Default|RecieveCollectableID (Variables|Default|GetPlayer%20Character%20Ref) (Variables|Default|GetCollectable%20ID))
    (Rendering|SetRenderCustomDepth (Variables|Default|GetItem) true)))

(event OnComponentEndOverlap(Box)
  (params (OverlappedComponent :type Primitive%20Component%20Object%20Reference) (OtherActor :type Actor%20Object%20Reference) (OtherComp :type Primitive%20Component%20Object%20Reference) (OtherBodyIndex :type Integer))
  ;[1 1 1] Is Player At Object
  (if (== OtherActor (Game|GetPlayerCharacter 0))
    ;[1 1 1] Can Press E
    (Input|DisableInput (Game|GetPlayerController 0))
    (Default|RecieveCollectableID (Variables|Default|GetPlayer%20Character%20Ref))
    (Rendering|SetRenderCustomDepth (Variables|Default|GetItem) false)))

(event EventHumanInteract
  (bind _audiodirector (Variables|Default|GetAudioDirector))
  ;[1 1 1] Collect Item
  (Utilities|FlowControl|Sequence
    (:then_0
      (Development|PrintString "You grabbed Item"))
    (:then_1
      (switch int (Variables|Default|GetWhichItem?)
        (:0
          (Default|GrabItem1 _audiodirector))
        (:1
          (Default|GrabItem2 _audiodirector))
        (:2
          (Default|GrabItem3 _audiodirector))
        (:3
          (Default|GrabItem4 _audiodirector))
        (:4
          (Default|GrabItem5 _audiodirector))
        (:5
          (Default|GrabItem6 _audiodirector))))
    (:then_2
      (Actor|DestroyActor))))

(event EventBeginPlay
  (bind _outactors (Actor|GetAllActorsOfClass "/Game/FirstPerson/Blueprints/BP_FirstPersonCharacter.BP_FirstPersonCharacter_C"))
  (Variables|Default|SetPlayer%20Character%20Ref (Utilities|Array|Get(acopy) _outactors))
  (bind _outactors_2 (Actor|GetAllActorsOfClass "/Game/Ethan_BPs/CC/Harshbarger_AudioDirector_BP.Harshbarger_AudioDirector_BP_C"))
  (Variables|Default|SetAudioDirector (Utilities|Array|Get(acopy) _outactors_2)))

(fn ConstructionScript)