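; Bridge spawn Blueprint that makes a bridge appear when the player enters a trigger.
; Overlap of the Trigger by player character 0 makes the existing BridgePlacement component visible and enables its query and physics collision, rather than spawning anything.
; The construction script shows the bridge when SeeBridge is set, without changing its collision.
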(event OnComponentBeginOverlap(Trigger)
  (params (OverlappedComponent :type Primitive%20Component%20Object%20Reference) (OtherActor :type Actor%20Object%20Reference) (OtherComp :type Primitive%20Component%20Object%20Reference) (OtherBodyIndex :type Integer) (bFromSweep :type Boolean) (SweepResult :type Hit%20Result%20Structure%20%28by%20ref%29))
  (bind _bridgeplacement (Variables|Default|GetBridgePlacement))
  (if (== OtherActor (Game|GetPlayerCharacter 0))
    (Rendering|SetVisibility _bridgeplacement true false)
    (Collision|SetCollisionEnabled _bridgeplacement "QueryAndPhysics")))

(fn ConstructionScript
  (if (Variables|Default|GetSeeBridge?)
    (Rendering|SetVisibility (Variables|Default|GetBridgePlacement) true false)))