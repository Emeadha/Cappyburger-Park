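; PushBP is an actor Blueprint that checks whether the player is positioned to push it.
; Its Can Push function runs a short visibility line trace from the player character's location along its forward vector, ignoring the player.
; It returns true only when that trace hits this actor.
; The Blueprint performs no movement itself, and its construction script is empty.
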(fn ConstructionScript)

(fn CanPush
  (bind _returnvalue (Game|GetPlayerCharacter 0))
  (bind _returnvalue_2 (Transformation|GetActorLocation _returnvalue))
  (bind (_outhit _returnvalue_3) (Collision|LineTraceByChannel _returnvalue_2 (+ _returnvalue_2 (* (Transformation|GetActorForwardVector _returnvalue) 1e+02)) "TraceTypeQuery1" false (Utilities|Array|MakeArray _returnvalue) "None" false))
  (if _returnvalue_3
    (if (== (.HitActor (Collision|BreakHitResult _outhit)) self)
      (return true)
      (else
        (return false)))
    (else
      (return false))))