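; World helicopter Blueprint that flies a Helicopter component along its Spline.
; Each Tick advances the distance along the spline by SplineSpeed times delta time and sets the helicopter's relative transform from that local-space point.
; Fixed height and yaw offsets adjust the placement while the component's scale is preserved.
; When Loop is set, the distance resets to zero after passing the spline's end.
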(event EventBeginPlay)

(event Collision|EventActorBeginOverlap
  (params (OtherActor :type Actor%20Object%20Reference)))

(event EventTick
  (params (DeltaSeconds :type Float%20%28single-precision%29))
  (Variables|Default|SetDistance%20along%20spline (+ (* DeltaSeconds (Variables|Default|GetSpline%20Speed)) (Variables|Default|GetDistance%20along%20spline)))
  (Transformation|SetRelativeTransform (Variables|Default|Gethelicopter) (Math|Transform|MakeTransform (Math|Vector|MakeVector (.x (.location (Spline|GetTransformatDistanceAlongSpline (Variables|Default|GetSpline) (Variables|Default|GetDistance%20along%20spline) "Local" false))) (.y (.location (Spline|GetTransformatDistanceAlongSpline (Variables|Default|GetSpline) (Variables|Default|GetDistance%20along%20spline) "Local" false))) (+ (.z (.location (Spline|GetTransformatDistanceAlongSpline (Variables|Default|GetSpline) (Variables|Default|GetDistance%20along%20spline) "Local" false))) -89.0)) (Math|Rotator|MakeRotator (.roll (.rotation (Spline|GetTransformatDistanceAlongSpline (Variables|Default|GetSpline) (Variables|Default|GetDistance%20along%20spline) "Local" false))) (.pitch (.rotation (Spline|GetTransformatDistanceAlongSpline (Variables|Default|GetSpline) (Variables|Default|GetDistance%20along%20spline) "Local" false))) (+ (.yaw (.rotation (Spline|GetTransformatDistanceAlongSpline (Variables|Default|GetSpline) (Variables|Default|GetDistance%20along%20spline) "Local" false))) -9e+01)) (Variables|/Script/Engine.SceneComponent|GetRelativeScale3D (Variables|Default|Gethelicopter))) false false)
  (if (Variables|Default|Getloop?)
    (if (> (Variables|Default|GetDistance%20along%20spline) (Spline|GetSplineLength (Variables|Default|GetSpline)))
      (Variables|Default|SetDistance%20along%20spline 0.0))))

(fn ConstructionScript)