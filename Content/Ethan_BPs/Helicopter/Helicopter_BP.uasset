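; Helicopter actor that flies along a fixed path on repeat and blinks a Cylinder component.
; On BeginPlay a timeline lerps the Helicopter component's relative location from a begin to an end point at a configurable play rate, restarting from the start after a short delay when finished.
; Tick runs a short Delay into a FlipFlop that toggles the Cylinder's visibility for a rapid flicker.
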(event Custom|MakeHelicoptorFly
  (bind _newtrack_0 (Timeline|HelicoptoerFly Play)
    (:Update
      (Transformation|SetRelativeLocation (Variables|Default|Gethelicopter) (Math|Vector|Lerp(Vector) (Variables|Default|GetHelicoptorBegin) (Variables|Default|GetHelicoptorEnd) _newtrack_0) false false))
    (:Finished
      (Utilities|FlowControl|Delay 0.2)
      (Timeline|HelicoptoerFly PlayFromStart))))

(event EventBeginPlay
  (CallFunction|MakeHelicoptorFly)
  (Components|Timeline|SetPlayRate (Variables|Default|GetHelicoptoerFly) (Variables|Default|GetMyPlayRate)))

(event Collision|EventActorBeginOverlap
  (params (OtherActor :type Actor%20Object%20Reference)))

(event EventTick
  (params (DeltaSeconds :type Float%20%28single-precision%29))
  (Utilities|FlowControl|Delay 0.01)
  (Utilities|FlowControl|FlipFlop
    (:A
      (Rendering|SetVisibility (Variables|Default|GetCylinder) true false))
    (:B
      (Rendering|SetVisibility (Variables|Default|GetCylinder) false false))))

(fn ConstructionScript)