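; Audio director actor that plays ambient music and character voice lines, paired with closed captions from a CC_BP widget it creates on BeginPlay.
; A delay-driven loop alternates two ambient tracks; the index resets before reaching the third.
; Character01 events trigger sounds (two unassigned) with captions.
; Talk steps through five captions, repeating the last and setting IntroDone, which unlocks WalkieCall's single caption.
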(event EventBeginPlay
  (Variables|Default|SetIntroDone? false)
  (Variables|Default|SetWalkie%20Selection 0)
  (Variables|Default|SetAmbient%20Selection 0)
  (Variables|Default|SetTalkInteger 0)
  (bind _returnvalue (UserInterface|CreateWidget "/Game/Ethan_BPs/CC/CC_BP.CC_BP_C"))
  (bind _output_get (Variables|Default|Setmyccwidget _returnvalue))
  (UserInterface|Viewport|AddtoViewport _output_get 0)
  ;[1 0.9938 0.7195] Ambient music
  (Utilities|FlowControl|Delay 3e+01 :!label _label)
  (switch int (Variables|Default|GetAmbient%20Selection)
    (:0
      (Audio|PlaySound2D "/Game/CAPPYPARK_SOUNDS/Music/AmbientMusic/A_walk_in_the_snow_01.A_walk_in_the_snow_01" 1.0 1.0 0.0 0 0)
      (Utilities|FlowControl|Delay 46.0))
    (:1
      (Audio|PlaySound2D "/Game/CAPPYPARK_SOUNDS/Music/AmbientMusic/A_peaceful_pine.A_peaceful_pine" 1.0 1.0 0.0 0 0)
      (Utilities|FlowControl|Delay 9e+01))
    (:2
      (Audio|PlaySound2D "/Game/CAPPYPARK_SOUNDS/Music/AmbientMusic/Vibin_Strums_01.Vibin_Strums_01" 1.0 1.0 0.0 0 0)
      (Utilities|FlowControl|Delay 47.0)))
  (Math|Integer|IncrementInt (Variables|Default|GetAmbient%20Selection)
    (:%20%20
      (if (>= (Variables|Default|GetAmbient%20Selection) 2)
        (Variables|Default|SetAmbient%20Selection 0)
        (goto _label)
        (else
          (goto _label))))))

(event Collision|EventActorBeginOverlap
  (params (OtherActor :type Actor%20Object%20Reference)))

(event EventTick
  (params (DeltaSeconds :type Float%20%28single-precision%29)))

(event EventCharacter01Line01
  ;[0.9694 1 0.07733] Character 1
  (Audio|PlaySound2D "/Game/CAPPYPARK_SOUNDS/This_is_a_test_1_01.This_is_a_test_1_01" 1.0 1.0 0.0 0 0)
  (Default|C1l1 (Variables|Default|Getmyccwidget)))

(event EventTalk
  (bind _myccwidget (Variables|Default|Getmyccwidget))
  (Math|Integer|IncrementInt (Variables|Default|GetTalkInteger)
    (:%20%20
      (switch int (Variables|Default|GetTalkInteger)
        (:1
          (Default|Talk1CC _myccwidget))
        (:2
          (Default|Talk2CC _myccwidget))
        (:3
          (Default|Talk3CC _myccwidget))
        (:4
          (Default|Talk4CC _myccwidget))
        (:5
          (Default|Talk5CC _myccwidget)
          (Variables|Default|SetIntroDone? true)
          (Variables|Default|SetTalkInteger 4))))))

(event EventCharacter01Line02
  ;[0.9694 1 0.07733] Character 1
  (Audio|PlaySound2D "/Game/CAPPYPARK_SOUNDS/Heagney_please_giv_gud_grade_01.Heagney_please_giv_gud_grade_01" 1.0 1.0 0.0 0 0)
  (Default|C1L2 (Variables|Default|Getmyccwidget)))

(event EventCharacter01Line03
  ;[0.9694 1 0.07733] Character 1
  (Audio|PlaySound2D 0 1.0 1.0 0.0 0 0)
  (Default|C1L3 (Variables|Default|Getmyccwidget)))

(event EventCharacter01Line04
  ;[0.9694 1 0.07733] Character 1
  (Audio|PlaySound2D 0 1.0 1.0 0.0 0 0)
  (Default|C1L4 (Variables|Default|Getmyccwidget)))

(event EventWalkieCall
  (if (Variables|Default|GetIntroDone?)
    (Math|Integer|IncrementInt (Variables|Default|GetWalkie%20Selection)
      (:%20%20
        (switch int (Variables|Default|GetWalkie%20Selection)
          (:1
            (Default|Walkie1CC (Variables|Default|Getmyccwidget))))))))

(fn ConstructionScript)