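; Animal encounter actor that shows a penguin, llama or fox, chosen by AnimalChoice, for the player to discover.
; A 0.1s Delay loop from BeginPlay stops the mystery ambience once Encountered is set.
; First box overlap plays a sound and the audio director's discovery line, then writes the character's unlock flag (true only for llama, false for penguin and fox).
; It then sets Encountered and destroys all three meshes after about ten seconds.
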(event OnComponentBeginOverlap(Box)
  (params (OverlappedComponent :type Primitive%20Component%20Object%20Reference) (OtherActor :type Actor%20Object%20Reference) (OtherComp :type Primitive%20Component%20Object%20Reference) (OtherBodyIndex :type Integer) (bFromSweep :type Boolean) (SweepResult :type Hit%20Result%20Structure%20%28by%20ref%29))
  (bind _audiodir (Variables|Default|GetAudioDir))
  (if (not (Variables|Default|GetEncountered?))
    (Audio|PlaySound2D "/Game/CAPPYPARK_SOUNDS/Music/Mystery_AmbienceETHAN.Mystery_AmbienceETHAN" 1.0 1.0 0.0 0 0)
    ;[1 1 1] Choose voice line
    (switch int (Variables|Default|GetAnimal%20Choice)
      (:0
        (Default|PengDiscovery _audiodir)
        ;[1 0.2746 0.466] Unlock Character
        (bind _asbp_first_person_character (Utilities|Casting|CastToBP_FirstPersonCharacter (Game|GetPlayerCharacter 0)))
        (Variables|/Game/FirstPerson/Blueprints/BP_FirstPersonCharacter.BP_FirstPersonCharacter_C|SetPengUnlocked _asbp_first_person_character false))
      (:1
        (Default|LlamaDiscovery _audiodir)
        (bind _asbp_first_person_character_2 (Utilities|Casting|CastToBP_FirstPersonCharacter (Game|GetPlayerCharacter 0)))
        (Variables|/Game/FirstPerson/Blueprints/BP_FirstPersonCharacter.BP_FirstPersonCharacter_C|SetLlamaUnlocked _asbp_first_person_character_2 true))
      (:2
        (Default|FoxDiscovery _audiodir)
        (bind _asbp_first_person_character_3 (Utilities|Casting|CastToBP_FirstPersonCharacter (Game|GetPlayerCharacter 0)))
        (Variables|/Game/FirstPerson/Blueprints/BP_FirstPersonCharacter.BP_FirstPersonCharacter_C|SetFoxUnlocked _asbp_first_person_character_3 false)))
    (Variables|Default|SetEncountered? true)
    (Utilities|FlowControl|Delay 10.2)
    (Components|DestroyComponent (Variables|Default|GetFox))))

(event EventBeginPlay
  (bind _outactors (Actor|GetAllActorsOfClass "/Game/Ethan_BPs/CC/Harshbarger_AudioDirector_BP.Harshbarger_AudioDirector_BP_C"))
  (Variables|Default|SetAudioDir (Utilities|Array|Get(acopy) _outactors))
  (switch int (Variables|Default|GetAnimal%20Choice)
    (:0
      ;[1 1 1] Choose which model visible
      (Rendering|SetVisibility (Variables|Default|GetMesh_Penguin) true false))
    (:1
      (Rendering|SetVisibility (Variables|Default|GetLlama) true false))
    (:2
      (Rendering|SetVisibility (Variables|Default|GetFox) true false)))
  ;[1 0.5571 0.4062] ambient noise
  (if (Variables|Default|GetEncountered?) :!label _label
    (Audio|Components|Audio|Stop (Variables|Default|GetMystery_AmbienceETHAN))
    (else
      (Utilities|FlowControl|Delay 0.1)
      (goto _label))))

(fn ConstructionScript)