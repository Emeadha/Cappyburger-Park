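; Harshbarger sound trigger actor that plays audio when the player character enters its box.
; Flags decide whether it fires only when the exit count equals a target, on every entry, or just once; end overlap updates the count and triggered state.
; With CC on, it messages HarshBAudioDirector to play one of four Character01 lines by selection; otherwise it plays two 2D sounds directly, bypassing the director.
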(event OnComponentBeginOverlap(Box)
  (params (OverlappedComponent :type Primitive%20Component%20Object%20Reference) (OtherActor :type Actor%20Object%20Reference) (OtherComp :type Primitive%20Component%20Object%20Reference) (OtherBodyIndex :type Integer) (bFromSweep :type Boolean) (SweepResult :type Hit%20Result%20Structure%20%28by%20ref%29))
  (bind _harshb_audiodirector (Variables|Default|GetHarshB_AudioDirector))
  ;[1 1 1] Comment
  ;[1 1 1] Checks If Player
  (if (== OtherActor (Game|GetPlayerCharacter 0))
    ;[1 0.1499 0.3922] Multiple Cross?
    (if (Variables|Default|GetPlay%20On%20Multiple%20Cross?)
      ;[0.2944 1 0.9002] Times To Trigger
      (if (== (Variables|Default|GetTimes%202%20Trigger) (Variables|Default|GetTimes%20Touched))
        (if (Variables|Default|GetCC?) :!label _label
          ;[0.4651 0.4242 1] Send Audio selection to manager
          (switch int (Variables|Default|GetCC%20Selection)
            (:0
              (Class|HarshbargerBPI|Character01Line01(Message) _harshb_audiodirector))
            (:1
              (Class|HarshbargerBPI|Character01Line02(Message) _harshb_audiodirector))
            (:2
              (Class|HarshbargerBPI|Character01Line03(Message) _harshb_audiodirector))
            (:3
              (Class|HarshbargerBPI|Character01Line04(Message) _harshb_audiodirector)))
          (else
            ;[1 0.4113 0.2365] Plays sound, no CC, no Audio Manager
            (Audio|PlaySound2D (Variables|Default|GetNO%20CC%20Sound%201) 1.0 1.0 0.0 0 0)
            (Audio|PlaySound2D (Variables|Default|GetNO%20CC%20Sound%202) 1.0 1.0 0.0 0 0))))
      (else
        ;[1 0.6149 0.4532] Happens More Than Once
        (if (Variables|Default|GetHappens%20More%20Than%20Once?)
          (goto _label)
          (else
            ;[0.3444 0.5153 1] Checks If Already Triggered
            (if (not (Variables|Default|GetAlready%20Triggered?))
              (goto _label))))))))

(event OnComponentEndOverlap(Box)
  (params (OverlappedComponent :type Primitive%20Component%20Object%20Reference) (OtherActor :type Actor%20Object%20Reference) (OtherComp :type Primitive%20Component%20Object%20Reference) (OtherBodyIndex :type Integer))
  ;[0.6013 1 0.6231] End Overlap
  ;;[1 1 1] Checks If Player
  (if (== OtherActor (Game|GetPlayerCharacter 0))
    (Math|Integer|IncrementInt (Variables|Default|GetTimes%20Touched)
      (:%20%20
        (Variables|Default|SetAlready%20Triggered? true)))))

(event EventBeginPlay
  ;[0.2737 0.315 1] Default Values
  (Variables|Default|SetAlready%20Triggered? false)
  (Variables|Default|SetTimes%20Touched 0))

(fn ConstructionScript)