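; Ice surface trigger that makes BP_FirstPersonCharacter slide by zeroing ground friction and walking braking while inside its box.
; For the penguin (CharValue 2), it also forces constant-speed movement along a 90-degree grid with a hard-coded yaw offset.
; The camera yaw follows that snapped direction with control rotation and player input disabled.
; Leaving the box restores fixed friction and braking values, camera control and input.
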(event OnComponentBeginOverlap(Box)
  (params (OverlappedComponent :type Primitive%20Component%20Object%20Reference) (OtherActor :type Actor%20Object%20Reference) (OtherComp :type Primitive%20Component%20Object%20Reference) (OtherBodyIndex :type Integer) (bFromSweep :type Boolean) (SweepResult :type Hit%20Result%20Structure%20%28by%20ref%29))
  (bind _asbp_first_person_character (Utilities|Casting|CastToBP_FirstPersonCharacter OtherActor))
  (Variables|/Script/Engine.CharacterMovementComponent|SetGroundFriction (Variables|/Script/Engine.Character|GetCharacterMovement _asbp_first_person_character) 0.0)
  (Variables|/Script/Engine.CharacterMovementComponent|SetBrakingDecelerationWalking (Variables|/Script/Engine.Character|GetCharacterMovement _asbp_first_person_character) 0.0)
  (bind _asbp_first_person_character_2 (Utilities|Casting|CastToBP_FirstPersonCharacter (Game|GetPlayerCharacter 0)))
  ;[0.269 0.501 1] If player == penguin
  (bind _asbp_first_person_character_3 (Utilities|Casting|CastToBP_FirstPersonCharacter (Game|GetPlayerCharacter 0)))
  (if (== (Variables|/Game/FirstPerson/Blueprints/BP_FirstPersonCharacter.BP_FirstPersonCharacter_C|GetCharValue _asbp_first_person_character_3) 2)
    (Variables|/Script/Engine.MovementComponent|SetVelocity (Variables|/Script/Engine.Character|GetCharacterMovement _asbp_first_person_character) (Math|Vector|MakeVector (* (Math|Trig|Cos(Degrees) (+ (Math|Conversions|ToFloat(Integer) (* (Math|Float|Round (/ (+ (Class|KismetMathLibrary|DegAtan2 (.Y (Math|Vector|BreakVector (Variables|/Script/Engine.MovementComponent|GetVelocity (Variables|/Script/Engine.Character|GetCharacterMovement _asbp_first_person_character)))) (.X (Math|Vector|BreakVector (Variables|/Script/Engine.MovementComponent|GetVelocity (Variables|/Script/Engine.Character|GetCharacterMovement _asbp_first_person_character))))) -55.901304) 9e+01)) 90)) 34.098696)) 5e+02) (* (Math|Trig|Sin(Degrees) (+ (Math|Conversions|ToFloat(Integer) (* (Math|Float|Round (/ (+ (Class|KismetMathLibrary|DegAtan2 (.Y (Math|Vector|BreakVector (Variables|/Script/Engine.MovementComponent|GetVelocity (Variables|/Script/Engine.Character|GetCharacterMovement _asbp_first_person_character)))) (.X (Math|Vector|BreakVector (Variables|/Script/Engine.MovementComponent|GetVelocity (Variables|/Script/Engine.Character|GetCharacterMovement _asbp_first_person_character))))) -55.901304) 9e+01)) 90)) 34.098696)) 5e+02) (.Z (Math|Vector|BreakVector (Variables|/Script/Engine.MovementComponent|GetVelocity (Variables|/Script/Engine.Character|GetCharacterMovement _asbp_first_person_character))))))
    (Variables|/Script/Engine.CameraComponent|SetbUsePawnControlRotation (Variables|/Game/FirstPerson/Blueprints/BP_FirstPersonCharacter.BP_FirstPersonCharacter_C|GetFirstPersonCamera _asbp_first_person_character) false)
    (Transformation|SetWorldRotation (Variables|/Game/FirstPerson/Blueprints/BP_FirstPersonCharacter.BP_FirstPersonCharacter_C|GetFirstPersonCamera _asbp_first_person_character) (Math|Rotator|MakeRotator 0.0 0.0 (+ (Math|Conversions|ToFloat(Integer) (* (Math|Float|Round (/ (+ (Class|KismetMathLibrary|DegAtan2 (.Y (Math|Vector|BreakVector (Variables|/Script/Engine.MovementComponent|GetVelocity (Variables|/Script/Engine.Character|GetCharacterMovement _asbp_first_person_character)))) (.X (Math|Vector|BreakVector (Variables|/Script/Engine.MovementComponent|GetVelocity (Variables|/Script/Engine.Character|GetCharacterMovement _asbp_first_person_character))))) -55.901304) 9e+01)) 90)) 34.098696)) false false)
    (Input|DisableInput _asbp_first_person_character_2 (Game|GetPlayerController 0))))

(event OnComponentEndOverlap(Box)
  (params (OverlappedComponent :type Primitive%20Component%20Object%20Reference) (OtherActor :type Actor%20Object%20Reference) (OtherComp :type Primitive%20Component%20Object%20Reference) (OtherBodyIndex :type Integer))
  (bind _asbp_first_person_character (Utilities|Casting|CastToBP_FirstPersonCharacter OtherActor))
  (Variables|/Script/Engine.CharacterMovementComponent|SetGroundFriction (Variables|/Script/Engine.Character|GetCharacterMovement _asbp_first_person_character) 8.0)
  (Variables|/Script/Engine.CharacterMovementComponent|SetBrakingDecelerationWalking (Variables|/Script/Engine.Character|GetCharacterMovement _asbp_first_person_character) 2048.0)
  (bind _asbp_first_person_character_2 (Utilities|Casting|CastToBP_FirstPersonCharacter (Game|GetPlayerCharacter 0)))
  (Variables|/Script/Engine.CameraComponent|SetbUsePawnControlRotation (Variables|/Game/FirstPerson/Blueprints/BP_FirstPersonCharacter.BP_FirstPersonCharacter_C|GetFirstPersonCamera _asbp_first_person_character_2) true)
  (Input|EnableInput _asbp_first_person_character_2 (Game|GetPlayerController 0)))

(fn ConstructionScript)