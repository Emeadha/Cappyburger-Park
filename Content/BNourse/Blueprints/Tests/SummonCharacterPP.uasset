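; Test trigger actor that summons a Simple3PActor at the player character's position.
; The first time the player overlaps its Box, a DoOnce gate spawns the actor regardless of collision, lowered by a hardcoded vertical offset, then matches the player's rotation.
; GetActiveChar is an empty stub.
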(event OnComponentBeginOverlap(Box)
  (params (OverlappedComponent :type Primitive%20Component%20Object%20Reference) (OtherActor :type Actor%20Object%20Reference) (OtherComp :type Primitive%20Component%20Object%20Reference) (OtherBodyIndex :type Integer) (bFromSweep :type Boolean) (SweepResult :type Hit%20Result%20Structure%20%28by%20ref%29))
  (bind _returnvalue (Game|GetPlayerCharacter 0))
  (if (== OtherActor _returnvalue)
    (Utilities|FlowControl|DoOnce false
      (:Completed
        (bind _returnvalue_2 (Game|SpawnActorfromClass "/Game/BNourse/Blueprints/Simple3PActor.Simple3PActor_C" (Math|Conversions|ToTransform(Vector) (- (Transformation|GetActorLocation _returnvalue) "0.000000,0.000000,98.150000")) "AlwaysSpawn" "MultiplyWithRoot" 0 0))
        (Transformation|SetActorRotation _returnvalue_2 (Transformation|GetActorRotation _returnvalue))))))

(event EventBeginPlay)

(event Collision|EventActorBeginOverlap
  (params (OtherActor :type Actor%20Object%20Reference)))

(event EventTick
  (params (DeltaSeconds :type Float%20%28single-precision%29)))

(fn ConstructionScript)

(fn GetActiveChar
  (return))