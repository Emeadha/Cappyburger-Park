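; Fence gate actor that procedurally builds a metal fence and can swing open.
; The construction script tiles instanced frame and bar meshes from Length, Height and TileSize.
; FenceOpen plays a timeline that lerps the actor's relative rotation from start to end.
; HumanInteract checks box overlap and the player's fuse count, one to four, but its DoOnce branches trigger nothing, including FenceOpen.
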(event EventBeginPlay)

(event Collision|EventActorBeginOverlap
  (params (OtherActor :type Actor%20Object%20Reference)))

(event EventTick
  (params (DeltaSeconds :type Float%20%28single-precision%29)))

(event EventFenceOpen
  (bind _newtrack_0 (Timeline|Timeline Play)
    (:Update
      (Transformation|SetActorRelativeRotation (Math|Rotator|Lerp(Rotator) (Variables|Default|GetStartingRotate) (Variables|Default|GetEndRotate) _newtrack_0)))))

(event EventHumanInteract
  (if (Collision|IsOverlappingActor (Variables|Default|Getboxcollision) (Game|GetPlayerCharacter 0) :!class /Script/Engine.PrimitiveComponent)
    (bind _asbp_first_person_character (Utilities|Casting|CastToBP_FirstPersonCharacter (Game|GetPlayerCharacter 0)))
    (if (== (Variables|/Game/FirstPerson/Blueprints/BP_FirstPersonCharacter.BP_FirstPersonCharacter_C|GetFuses _asbp_first_person_character) 1)
      (Utilities|FlowControl|DoOnce false)
      (elif (== (Variables|/Game/FirstPerson/Blueprints/BP_FirstPersonCharacter.BP_FirstPersonCharacter_C|GetFuses _asbp_first_person_character) 2)
        (Utilities|FlowControl|DoOnce false)
        (elif (== (Variables|/Game/FirstPerson/Blueprints/BP_FirstPersonCharacter.BP_FirstPersonCharacter_C|GetFuses _asbp_first_person_character) 3)
          (Utilities|FlowControl|DoOnce false)
          (elif (== (Variables|/Game/FirstPerson/Blueprints/BP_FirstPersonCharacter.BP_FirstPersonCharacter_C|GetFuses _asbp_first_person_character) 4)
            (Utilities|FlowControl|DoOnce false)))))))

(fn ConstructionScript
  (bind _tilesize (Variables|Default|GetTileSize))
  (bind _metalfenceh (Variables|Default|GetMetalFenceH))
  (bind _tilesize_2 (Variables|Default|GetTileSize))
  (bind _metalfencev (Variables|Default|GetMetalFenceV))
  (bind _tilesize_3 (Variables|Default|GetTileSize))
  (for _index (range 1 (Variables|Default|GetHeight))
    (Components|InstancedStaticMesh|AddInstance _metalfencev (Math|Conversions|ToTransform(Vector) (Math|Vector|MakeVector (Math|Conversions|ToFloat(Integer) (- _tilesize 15)) 0.0 (Math|Conversions|ToFloat(Integer) (* _index _tilesize)))) false)
    (Components|InstancedStaticMesh|AddInstance _metalfencev (Math|Conversions|ToTransform(Vector) (Math|Vector|MakeVector (Math|Conversions|ToFloat(Integer) (+ (* (Variables|Default|GetLength) _tilesize) 15)) 0.0 (Math|Conversions|ToFloat(Integer) (* _index _tilesize)))) false))
  (for _index_2 (range 1 (Variables|Default|GetLength))
    (Components|InstancedStaticMesh|AddInstance _metalfenceh (Math|Conversions|ToTransform(Vector) (Math|Vector|MakeVector (Math|Conversions|ToFloat(Integer) (* _index_2 _tilesize_2)) 0.0 (Math|Conversions|ToFloat(Integer) (- _tilesize_2 15)))) false)
    (Components|InstancedStaticMesh|AddInstance _metalfenceh (Math|Conversions|ToTransform(Vector) (Math|Vector|MakeVector (Math|Conversions|ToFloat(Integer) (* _index_2 _tilesize_2)) 0.0 (Math|Conversions|ToFloat(Integer) (+ (* (Variables|Default|GetHeight) _tilesize_2) 15)))) false)
    (for _index_3 (range 1 (Variables|Default|GetHeight))
      (Components|InstancedStaticMesh|AddInstance (Variables|Default|GetMetalBars) (Math|Conversions|ToTransform(Vector) (Math|Vector|MakeVector (Math|Conversions|ToFloat(Integer) (* _index_2 _tilesize_3)) 0.0 (Math|Conversions|ToFloat(Integer) (* _index_3 _tilesize_3)))) false))))